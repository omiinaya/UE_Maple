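; BP_ClimbingBase is a base climbable object that tells players when they are within range to climb it.
; Its CollisionBox overlap events run their logic only on the server and respond only to actors tagged Player.
; The player reference is fetched by message, then sent CanClimbMessage: true with this object on entry, false on exit.
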(event OnComponentBeginOverlap(CollisionBox)
  (params (OverlappedComponent :type Primitive%20Component%20Object%20Reference) (OtherActor :type Actor%20Object%20Reference) (OtherComp :type Primitive%20Component%20Object%20Reference) (OtherBodyIndex :type Integer) (bFromSweep :type Boolean) (SweepResult :type Hit%20Result%20Structure%20%28by%20ref%29))
  ;[1 1 1] Sets "Can Climb" depending on if the player is colliding with the CollisionBox or not.
  (Networking|SwitchHasAuthority
    (:Authority
      (if (Actor|ActorHasTag OtherActor "Player")
        (bind _player (Class|INTPlayerBase|GetPlayerRef(Message) OtherActor))
        (Class|INTPlayerBase|CanClimb(Message) _player true self)))))

(event OnComponentEndOverlap(CollisionBox)
  (params (OverlappedComponent :type Primitive%20Component%20Object%20Reference) (OtherActor :type Actor%20Object%20Reference) (OtherComp :type Primitive%20Component%20Object%20Reference) (OtherBodyIndex :type Integer))
  ;[1 1 1] Sets "Can Climb" depending on if the player is colliding with the CollisionBox or not.
  (Networking|SwitchHasAuthority
    (:Authority
      (if (Actor|ActorHasTag OtherActor "Player")
        (bind _player (Class|INTPlayerBase|GetPlayerRef(Message) OtherActor))
        (Class|INTPlayerBase|CanClimb(Message) _player false)))))

(fn ConstructionScript)