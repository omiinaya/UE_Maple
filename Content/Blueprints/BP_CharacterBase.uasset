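; Base character Blueprint that shows floating damage numbers above whichever player or enemy takes damage.
; DisplayFloatingText forwards to an SRV event, which spawns a BP_FloatingText actor just above the damaged actor.
; The text type selects color, icon and damage amount, read from the damaged actor through enemy or player reference getters.
; GetCharacterRef returns the character itself.
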(event Custom|SRV_DisplayFloatingText
  (params (DamagedActor :type Actor%20Object%20Reference) (FloatingTextType :type E_FloatingTextType%20Enum :default "NewEnumerator0"))
  ;[1 1 1 1 20] Floating text playing above enemy or player depending on who's getting damaged. The damaged actor is set through the AnyDamage of the player and enemy.
  (bind _output_get (Variables|Default|SetDamagedActor DamagedActor))
  (bind _returnvalue (Game|SpawnActorfromClass "/Game/Blueprints/BP_FloatingText.BP_FloatingText_C" (Math|Transform|MakeTransform (Math|Vector|MakeVector (.X (Math|Vector|BreakVector (Transformation|GetActorLocation _output_get))) (.Y (Math|Vector|BreakVector (Transformation|GetActorLocation _output_get))) (+ (.Z (Math|Vector|BreakVector (Transformation|GetActorLocation _output_get))) 3e+01))) "AdjustIfPossibleButAlwaysSpawn" 0 0))
  (bind _output_get_2 (Variables|Default|SetFloatingText _returnvalue))
  (switch Utilities|FlowControl|Switch|SwitchonE_FloatingTextType FloatingTextType
    (:NewEnumerator0
      (bind _enemy (Class|INTEnemyBase|GetEnemyRef(Message) (Variables|Default|GetDamagedActor)))
      (Default|DisplayFloatingText _output_get_2 (Utilities|Text|ToText(Float) (Variables|/Game/Blueprints/Enemy/BP_EnemyBase.BP_EnemyBase_C|GetPlayerDamageAmount _enemy) "HalfToEven") "(R=0.500000,G=0.790460,B=1.000000,A=1.000000)" "/Game/UI/Images/IMG_Sword.IMG_Sword"))
    (:NewEnumerator1
      (bind _player (Class|INTPlayerBase|GetPlayerRef(Message) (Variables|Default|GetDamagedActor)))
      (Default|DisplayFloatingText _output_get_2 (Utilities|Text|ToText(Float) (Variables|/Game/Blueprints/Player/BP_PlayerBase.BP_PlayerBase_C|GetEnemyDamageAmount _player) "HalfToEven") "(R=1.000000,G=0.500000,B=0.562874,A=1.000000)" "/Game/UI/Images/IMG_Blood.IMG_Blood"))))

(event EventDisplayFloatingText
  (params (DamagedActor :type Actor%20Object%20Reference) (FloatingTextType :type E_FloatingTextType%20Enum :default "NewEnumerator0"))
  ;[1 1 1 1 20] Floating text playing above enemy or player depending on who's getting damaged. The damaged actor is set through the AnyDamage of the player and enemy.
  (CallFunction|SRVDisplayFloatingText DamagedActor FloatingTextType))

(fn ConstructionScript)

(fn GetCharacterRef
  (return self))