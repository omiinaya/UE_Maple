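; Player controller for a Maplestory game that handles character selection, player spawning and HUD updates.
; On begin play it creates the character selection and main widgets through a client event, showing only the selection screen.
; Character choice goes through a server event to the GameMode via interface message, and SpawnPlayer spawns and possesses the pawn.
; Health and experience updates are relayed through client events to the main widget.
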(event Custom|CL_UpdateHealthBar
  (params (Percent :type Float%20%28single-precision%29) (EnemyName :type String))
  ;[1 1 1] Updating the health and experience bars
  (Default|UpdateHealth (Variables|WidgetBlueprint|GetWB_Main) Percent EnemyName))

(event Custom|CL_InitializeWidgets
  ;[1 1 1] Initializing widgets
  (bind _returnvalue (UserInterface|CreateWidget "/Game/UI/WB_CharacterSelection.WB_CharacterSelection_C"))
  (bind _output_get (Variables|WidgetBlueprint|SetWB_CharacterSelection _returnvalue))
  (UserInterface|Viewport|AddtoViewport _output_get 0)
  (bind _returnvalue_2 (UserInterface|CreateWidget "/Game/UI/WB_Main.WB_Main_C"))
  (Variables|WidgetBlueprint|SetWB_Main _returnvalue_2))

(event Custom|CL_UpdateExperience
  (params (PlayerInfo :type ST%20Player%20Info%20Structure))
  ;[1 1 1] Updating the health and experience bars
  (Default|UpdateExperience (Variables|WidgetBlueprint|GetWB_Main) PlayerInfo))

(event Custom|SRV_SelectCharacter
  (params (Player :type Actor%20Class%20Reference) (SpawnLocation :type Vector))
  ;[1 1 1] Selecting and spawning the player character
  (bind _gamemode (Class|INTGameMode|GetGameModeRef(Message) (Game|GetGameMode)))
  (Class|INTGameMode|RequestSpawnPlayer(Message) _gamemode self Player SpawnLocation))

(event EventUpdateHealthBar
  (params (Percent :type Float%20%28double-precision%29) (EnemyName :type String))
  ;[1 1 1] Updating the health and experience bars
  (CallFunction|CLUpdateHealthBar Percent EnemyName))

(event EventUpdateExperience
  (params (PlayerInfo :type ST%20Player%20Info%20Structure))
  ;[1 1 1] Updating the health and experience bars
  (CallFunction|CLUpdateExperience PlayerInfo))

(event EventBeginPlay
  ;[1 1 1] Begin Play - Initializing widgets
  (CallFunction|InitializeWidgets))

(event EventInitializeWidgets
  ;[1 1 1] Initializing widgets
  (CallFunction|CLInitializeWidgets))

(event EventSelectCharacter
  (params (Player :type Actor%20Class%20Reference) (SpawnLocation :type Vector :default "0, 0, 0"))
  ;[1 1 1] Selecting and spawning the player character
  (CallFunction|SRVSelectCharacter Player SpawnLocation))

(event EventSpawnPlayer
  (params (Player :type Actor%20Class%20Reference) (SpawnTransform :type Transform))
  ;[1 1 1] Selecting and spawning the player character
  (bind _returnvalue (Game|SpawnActorfromClass Player SpawnTransform "AdjustIfPossibleButAlwaysSpawn" 0 0))
  (bind _player (Class|INTPlayerBase|GetPlayerRef(Message) _returnvalue))
  (Pawn|Possess _player))

(fn ConstructionScript)

(fn GetPlayerControllerRef
  (return self))