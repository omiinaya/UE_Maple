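; Base class for replicated 2D sprite enemies, driven by an AnimalInfo struct for stats, flipbooks and death sound.
; When hit, it pauses its behavior tree, then either chases the attacker in back-and-forth passes or awards experience, fades out and respawns at a random navmesh point after a delay.
; A looping timer damages overlapping non-god-mode players.
; Server events set state, and RepNotifies apply flipbooks, materials, fade color and respawn location.
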(event OnComponentBeginOverlap(Collision)
  (params (OverlappedComponent :type Primitive%20Component%20Object%20Reference) (OtherActor :type Actor%20Object%20Reference) (OtherComp :type Primitive%20Component%20Object%20Reference) (OtherBodyIndex :type Integer) (bFromSweep :type Boolean) (SweepResult :type Hit%20Result%20Structure%20%28by%20ref%29))
  ;[1 1 1] Apply damage continuously through the timer when player is within the Collision box. If outside, stop applying continuous damage.
  (Networking|SwitchHasAuthority
    (:Authority
      (if (Actor|ActorHasTag OtherActor "Player")
        (CallFunction|StartApplyDamage true)))))

(event OnComponentEndOverlap(Collision)
  (params (OverlappedComponent :type Primitive%20Component%20Object%20Reference) (OtherActor :type Actor%20Object%20Reference) (OtherComp :type Primitive%20Component%20Object%20Reference) (OtherBodyIndex :type Integer))
  ;[1 1 1] Apply damage continuously through the timer when player is within the Collision box. If outside, stop applying continuous damage.
  (Networking|SwitchHasAuthority
    (:Authority
      (if (Actor|ActorHasTag OtherActor "Player")
        (CallFunction|StartApplyDamage false)))))

(event Custom|SRV_SetMovementState
  (params (MovementState :type E_MovementState%20Enum :default "NewEnumerator0"))
  ;[1 1 1] Sets the movement state.
  (Variables|Default|SetMovementState MovementState))

(event Custom|SRV_StartApplyDamage
  (params (bApplyDamage :type Boolean))
  ;[1 1 1] Apply damage continuously through the timer when player is within the Collision box. If outside, stop applying continuous damage.
  (if bApplyDamage
    (bind _returnvalue (Utilities|Time|SetTimerbyEvent (delegate Custom|ApplyDamage) 0.1 true))
    (Variables|Default|SetApplyDamageHandle _returnvalue)
    (else
      (Utilities|Time|ClearandInvalidateTimerbyHandle (Variables|Default|GetApplyDamageHandle)))))

(event Custom|ApplyDamage
  ;[1 1 1] Apply damage continuously through the timer when player is within the Collision box. If outside, stop applying continuous damage.
  (for _array_element (Collision|GetOverlappingActors "/Game/Blueprints/Player/BP_PlayerBase.BP_PlayerBase_C" :!class /Script/Engine.Actor)
    (bind _player (Class|INTPlayerBase|GetPlayerRef(Message) _array_element))
    (if (not (Variables|/Game/Blueprints/Player/BP_PlayerBase.BP_PlayerBase_C|GetbGodMode _player))
      (Game|Damage|ApplyDamage _player (Utilities|Struct|BreakST_AnimalInfo (Variables|Default|GetAnimalInfo)) (Pawn|GetController) 0 "/Script/Engine.DamageType"))))

(event Custom|SRV_Death
  (params (bIsDead :type Boolean))
  ;[1 1 1] Enemy Death
  (bind _output_get (Variables|Default|SetbIsDead bIsDead))
  (if _output_get
    (CallFunction|MCDeath (Utilities|Struct|BreakST_AnimalInfo (Variables|Default|GetAnimalInfo)) (Transformation|GetActorLocation))))

(event Custom|SRV_Respawn
  ;[1 1 1] Sets the enemy respawn location at a random point on the navigation mesh.
  (bind _returnvalue (Actor|GetActorOfClass "/Script/NavigationSystem.NavMeshBoundsVolume"))
  (Variables|Default|SetSpawnLocation (Math|Vector|MakeVector (.X (Math|Vector|BreakVector (.RandomLocation (AI|Navigation|GetRandomReachablePointinRadius (Transformation|GetActorLocation) (.X (Math|Vector|BreakVector (.BoxExtent (Collision|GetActorBounds _returnvalue false false)))) 0 0)))) (.Y (Math|Vector|BreakVector (Transformation|GetActorLocation))) (+ (.Z (Math|Vector|BreakVector (.RandomLocation (AI|Navigation|GetRandomReachablePointinRadius (Transformation|GetActorLocation) (.X (Math|Vector|BreakVector (.BoxExtent (Collision|GetActorBounds _returnvalue false false)))) 0 0)))) 2e+01))))

(event Custom|SRV_ActorFade
  (params (bFade :type Boolean))
  ;[1 1 1] Actor fading when dead
  (bind _output_get (Variables|Default|SetbActorFade bFade))
  (if _output_get
    (bind _fadealpha (Timeline|FadingActor PlayFromStart)
      (:Update
        (Variables|Default|SetActorFadeColor (Math|Color|Lerp(LinearColor) "(R=1.000000,G=1.000000,B=1.000000,A=1.000000)" "(R=1.000000,G=1.000000,B=1.000000,A=0.000000)" _fadealpha)))
      (:Finished
        (if (not (Variables|Default|GetbActorFade))
          (CallFunction|Death false)
          (CallFunction|RestartBehaviorTree))))
    (else
      (Timeline|FadingActor ReverseFromEnd))))

(event Custom|MC_Death
  (params (EnemyDeathSFX :type Sound%20Base%20Object%20Reference) (Location :type Vector))
  ;[1 1 1] Enemy Death
  (Audio|PlaySoundatLocation EnemyDeathSFX Location "0, 0, 0" 1.0 1.0 0.0 0 0 0 0))

(event Custom|CL_RestartBehaviorTree
  ;[1 1 1] Restarting the Behaviour Tree
  (Components|Movement|StopMovementImmediately (Variables|Character|GetCharacterMovement))
  (AI|Logic|StopLogic (Variables|/Script/AIModule.AIController|GetBrainComponent (AI|GetAIController self)) "")
  (bind _aicontroller (Class|INTAIController|GetAIControllerRef(Message) (AI|GetAIController self)))
  (Class|INTAIController|RunAITree(Message) _aicontroller))

(event EventSetMovementState
  (params (MovementState :type E_MovementState%20Enum :default "NewEnumerator0"))
  ;[1 1 1] Sets the movement state.
  (CallFunction|SRVSetMovementState MovementState))

(event Game|Damage|EventAnyDamage
  (params (Damage :type Float%20%28single-precision%29) (DamageType :type Damage%20Type%20Object%20Reference) (InstigatedBy :type Controller%20Object%20Reference) (DamageCauser :type Actor%20Object%20Reference))
  (bind _returnvalue (Transformation|GetActorLocation))
  (bind (_x _y _z) (Math|Vector|BreakVector _returnvalue))
  ;[1 1 1] Enemy receiving damage
  (Variables|Default|SetPlayerDamageAmount Damage)
  (CallFunction|DisplayFloatingText self "NewEnumerator0")
  (Variables|Default|SetPlayerController InstigatedBy)
  ;;[1 1 1] Sets the new enemy health after it has been damaged.
  (bind _structout (Utilities|Struct|SetmembersinST_AnimalInfo (Variables|Default|GetAnimalInfo) (Math|Float|Clamp(Float) (- (Utilities|Struct|BreakST_AnimalInfo (Variables|Default|GetAnimalInfo)) Damage) 0.0 (Utilities|Struct|BreakST_AnimalInfo (Variables|Default|GetAnimalInfo)))))
  (bind _output_get (Variables|Default|SetAnimalInfo _structout))
  ;;[1 1 1] Stops the enemy movement and behaviour tree and plays the hit animation.
  (Pawn|Components|CharacterMovement|SetMovementMode (Variables|Character|GetCharacterMovement) "MOVE_None" 0)
  (CallFunction|SetMovementState "NewEnumerator8")
  (AI|Logic|StopLogic (Variables|/Script/AIModule.AIController|GetBrainComponent (AI|GetAIController self)) "Hit")
  (Utilities|FlowControl|Delay (Class|PaperFlipbookComponent|GetFlipbookLength (Variables|Default|GetSprite)))
  ;;[1 1 1] Checks if enemy health is 0 or not (dead or not)
  (if (== (Utilities|Struct|BreakST_AnimalInfo _output_get) 0.0)
    (bind _player (Class|INTPlayerBase|GetPlayerRef(Message) (Pawn|GetControlledPawn (Variables|Default|GetPlayerController))))
    (Class|INTPlayerBase|AddExperience(Message) _player (Utilities|Struct|BreakST_AnimalInfo (Variables|Default|GetAnimalInfo)))
    (CallFunction|Death true)
    (Variables|/Script/Engine.PrimitiveComponent|SetbGenerateOverlapEvents (Variables|Default|GetHitbox) false)
    (Variables|/Script/Engine.PrimitiveComponent|SetbGenerateOverlapEvents (Variables|Default|GetCollision) false)
    (CallFunction|ActorFade true)
    (Utilities|FlowControl|Delay (Variables|Default|GetRespawnTimer))
    (bind _structout_2 (Utilities|Struct|SetmembersinST_AnimalInfo (Variables|Default|GetAnimalInfo) (Utilities|Struct|BreakST_AnimalInfo (Variables|Default|GetAnimalInfo))))
    (Variables|Default|SetAnimalInfo _structout_2)
    (Variables|/Script/Engine.PrimitiveComponent|SetbGenerateOverlapEvents (Variables|Default|GetHitbox) true)
    (Variables|/Script/Engine.PrimitiveComponent|SetbGenerateOverlapEvents (Variables|Default|GetCollision) true)
    (Pawn|Components|CharacterMovement|SetMovementMode (Variables|Character|GetCharacterMovement) "MOVE_Walking" 0)
    (CallFunction|SetMovementState "NewEnumerator1")
    (CallFunction|Respawn)
    (CallFunction|ActorFade false)
    (CallFunction|RestartBehaviorTree)
    (else
      (Pawn|Components|CharacterMovement|SetMovementMode (Variables|Character|GetCharacterMovement) "MOVE_Walking" 0)
      (CallFunction|SetMovementState "NewEnumerator1")
      (AI|AIMoveTo self (Transformation|GetActorLocation (Pawn|GetControlledPawn (Variables|Default|GetPlayerController))) (Pawn|GetControlledPawn (Variables|Default|GetPlayerController)) 2.0 true :!label _label
        (:OnSuccess
          (bind _player_2 (Class|INTPlayerBase|GetPlayerRef(Message) (Pawn|GetControlledPawn (Variables|Default|GetPlayerController))))
          (if (not (Variables|/Game/Blueprints/Player/BP_PlayerBase.BP_PlayerBase_C|GetbIsDead _player_2))
            (AI|AIMoveTo (AI|GetAIController self) (Math|Vector|MakeVector (+ _x (Math|Float|SelectFloat -125.0 125.0 (< (.X (Math|Vector|BreakVector (Transformation|GetActorLocation (Pawn|GetControlledPawn (Variables|Default|GetPlayerController))))) _x))) _y _z) 0 -1.0 "Default" "Enable" true true
              (:OnMoveFinished
                (goto _label)))
            (else
              (CallFunction|RestartBehaviorTree))))))))

(event EventStartApplyDamage
  (params (bApplyDamage :type Boolean))
  ;[1 1 1] Apply damage continuously through the timer when player is within the Collision box. If outside, stop applying continuous damage.
  (CallFunction|SRVStartApplyDamage bApplyDamage))

(event EventDeath
  (params (bIsDead :type Boolean))
  ;[1 1 1] Enemy Death
  (CallFunction|SRVDeath bIsDead))

(event EventRespawn
  ;[1 1 1] Sets the enemy respawn location at a random point on the navigation mesh.
  (CallFunction|SRVRespawn))

(event EventActorFade
  (params (bFade :type Boolean))
  ;[1 1 1] Actor fading when dead
  (CallFunction|SRVActorFade bFade))

(event EventRestartBehaviorTree
  ;[1 1 1] Restarting the Behaviour Tree
  (CallFunction|CLRestartBehaviorTree))

(fn ConstructionScript
  (|CallParentFunction))

(fn OnRepBIsMoving
  (bind _sprite (Variables|Default|GetSprite))
  (bind _animalinfo (Variables|Default|GetAnimalInfo))
  (bind (_name _health _maxhealth _damage _experience _idleanimation _moveanimation) (Utilities|Struct|BreakST_AnimalInfo _animalinfo))
  (if (not (Variables|Default|GetbIsMoving))
    (Sprite|SetFlipbook _sprite _idleanimation)
    (else
      (Sprite|SetFlipbook _sprite _moveanimation))))

(fn OnRepMovementState
  (bind _sprite (Variables|Default|GetSprite))
  (bind _animalinfo (Variables|Default|GetAnimalInfo))
  (bind (_experience _idleanimation _moveanimation _hitanimation _deathanimation) (Utilities|Struct|BreakST_AnimalInfo _animalinfo))
  (switch Utilities|FlowControl|Switch|SwitchonE_MovementState (Variables|Default|GetMovementState)
    (:NewEnumerator0
      (Sprite|SetFlipbook _sprite _idleanimation))
    (:NewEnumerator1
      (Sprite|SetFlipbook _sprite _moveanimation))
    (:NewEnumerator8
      (Sprite|SetFlipbook _sprite _hitanimation))
    (:NewEnumerator9
      (Sprite|SetFlipbook _sprite _deathanimation))))

(fn OnRepBIsDead
  (if (Variables|Default|GetbIsDead)
    (CallFunction|SetMovementState "NewEnumerator9")
    (Rendering|Material|SetMaterial (Variables|Default|GetSprite) 0 "/Paper2D/TranslucentUnlitSpriteMaterial.TranslucentUnlitSpriteMaterial")
    (else
      (Rendering|Material|SetMaterial (Variables|Default|GetSprite) 0 "/Paper2D/MaskedUnlitSpriteMaterial.MaskedUnlitSpriteMaterial"))))

(fn OnRepSpawnLocation
  (Transformation|SetActorLocation (Variables|Default|GetSpawnLocation) false false))

(fn OnRepActorFadeColor
  (Sprite|SetSpriteColor (Variables|Default|GetSprite) (Variables|Default|GetActorFadeColor)))

(fn GetEnemyRef
  (return self))